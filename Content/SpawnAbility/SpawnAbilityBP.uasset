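; SpawnAbilityBP is a spawner actor that places a random ability actor at its own location.
; On BeginPlay it picks a class from AbilitiesToSpawn, spawns it with itself as owner, stores it as CurrentAbility and applies a one-time local roll offset.
; The Respawn event clears that reference, waits RespawnTime, then spawns again unless a valid ability is already held.
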(event `self.ReceiveBeginPlay`
  (`self.CheckToSpawn`))

(event `/Game/SpawnAbility/Ineract/Spawner.Respawn`
  (set `self.CurrentAbility` null)
  (`KismetSystemLibrary.Delay` (`self.RespawnTime`))
  (`self.CheckToSpawn`))

(fn `AbilitySpawn`
  (bind _output_get (set `self.AbilityNumber` (`KismetMathLibrary.RandomIntegerInRange` 0 (- (`KismetArrayLibrary.Array_Length` (`self.AbilitiesToSpawn`)) 1))))
  (bind _returnvalue (`|SpawnActorFromClass` (`|GetArrayItem` (`self.AbilitiesToSpawn`) _output_get) (`KismetMathLibrary.MakeTransform` (`self.K2_GetActorLocation`) (`self.K2_GetActorRotation`)) "AlwaysSpawn" "OverrideRootScale" self null))
  (bind _output_get_2 (set `self.CurrentAbility` _returnvalue))
  (`self.K2_AddActorLocalRotation` _output_get_2 (* (`KismetMathLibrary.MakeRotator` (+ (`self.NewVar_0`) 1.0)) (`self.NewVar_1`)) false false))

(fn `CheckToSpawn`
  (`/Engine/EditorBlueprintResources/StandardMacros.IsValid` (`self.CurrentAbility`)
    (:`Is Valid`
      (`KismetSystemLibrary.PrintString` "Hello"))
    (:`Is Not Valid`
      (`self.AbilitySpawn`))))

(fn `UserConstructionScript`)